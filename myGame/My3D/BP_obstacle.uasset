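; BP_obstacle is a moving hazard that kills the third-person player on contact.
; A timeline loops by reversing on finish, driving the static mesh's relative Z position back and forth.
; Three trigger boxes repeat the same once-only logic: ragdoll the character, spawn an explosion, play a sound and show the Wasted widget.
; Each box then plays its own timeline as a delay before opening level_2.
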(event OnComponentBeginOverlap(Box)
  (params (OverlappedComponent :type Primitive%20Component%20Object%20Reference) (OtherActor :type Actor%20Object%20Reference) (OtherComp :type Primitive%20Component%20Object%20Reference) (OtherBodyIndex :type Integer) (bFromSweep :type Boolean) (SweepResult :type Hit%20Result%20Structure%20%28by%20ref%29))
  (bind _asbp_third_person_character (Utilities|Casting|CastToBP_ThirdPersonCharacter OtherActor))
  (Utilities|FlowControl|DoOnce false
    (:Completed
      (Default|Rgdol _asbp_third_person_character)
      (Effects|SpawnEmitteratLocation "/Game/StarterContent/Particles/P_Explosion.P_Explosion" (Transformation|GetActorLocation _asbp_third_person_character))
      (Audio|PlaySound2D "/Game/StarterContent/Audio/Collapse01.Collapse01" 1.0 1.0 0.0 0 0)
      (bind _returnvalue (UserInterface|CreateWidget "/Game/newenironment/Widgets/Wasted.Wasted_C"))
      (UserInterface|Viewport|AddtoViewport _returnvalue 0)
      (Timeline|Timeline_1 Play
        (:Finished
          (Game|OpenLevel(byName) "level_2"))))))

(event OnComponentBeginOverlap(Box1)
  (params (OverlappedComponent :type Primitive%20Component%20Object%20Reference) (OtherActor :type Actor%20Object%20Reference) (OtherComp :type Primitive%20Component%20Object%20Reference) (OtherBodyIndex :type Integer) (bFromSweep :type Boolean) (SweepResult :type Hit%20Result%20Structure%20%28by%20ref%29))
  (bind _asbp_third_person_character (Utilities|Casting|CastToBP_ThirdPersonCharacter OtherActor))
  (Utilities|FlowControl|DoOnce false
    (:Completed
      (Default|Rgdol _asbp_third_person_character)
      (Effects|SpawnEmitteratLocation "/Game/StarterContent/Particles/P_Explosion.P_Explosion" (Transformation|GetActorLocation _asbp_third_person_character))
      (Audio|PlaySound2D "/Game/StarterContent/Audio/Collapse01.Collapse01" 1.0 1.0 0.0 0 0)
      (bind _returnvalue (UserInterface|CreateWidget "/Game/newenironment/Widgets/Wasted.Wasted_C"))
      (UserInterface|Viewport|AddtoViewport _returnvalue 0)
      (Timeline|Timeline_0 Play
        (:Finished
          (Game|OpenLevel(byName) "level_2"))))))

(event OnComponentBeginOverlap(Box2)
  (params (OverlappedComponent :type Primitive%20Component%20Object%20Reference) (OtherActor :type Actor%20Object%20Reference) (OtherComp :type Primitive%20Component%20Object%20Reference) (OtherBodyIndex :type Integer) (bFromSweep :type Boolean) (SweepResult :type Hit%20Result%20Structure%20%28by%20ref%29))
  (bind _asbp_third_person_character (Utilities|Casting|CastToBP_ThirdPersonCharacter OtherActor))
  (Utilities|FlowControl|DoOnce false
    (:Completed
      (Default|Rgdol _asbp_third_person_character)
      (Effects|SpawnEmitteratLocation "/Game/StarterContent/Particles/P_Explosion.P_Explosion" (Transformation|GetActorLocation _asbp_third_person_character))
      (Audio|PlaySound2D "/Game/StarterContent/Audio/Collapse01.Collapse01" 1.0 1.0 0.0 0 0)
      (bind _returnvalue (UserInterface|CreateWidget "/Game/newenironment/Widgets/Wasted.Wasted_C"))
      (UserInterface|Viewport|AddtoViewport _returnvalue 0)
      (Timeline|Timeline_2 Play
        (:Finished
          (Game|OpenLevel(byName) "level_2"))))))

(event Custom|PlayForward
  (bind (_direction _newtrack_0) (Timeline|Timeline PlayFromStart)
    (:Update
      (Transformation|SetRelativeLocation (Variables|Default|GetStaticMesh) (Math|Vector|MakeVector 0.0 0.0 (* _newtrack_0 1e+02)) false false))
    (:Finished
      (if (Utilities|Enum|Equal(Enum) _direction "Forward")
        (CallFunction|PlayBackward)
        (else
          (CallFunction|PlayForward))))))

(event Custom|PlayBackward
  (bind (_direction _newtrack_0) (Timeline|Timeline ReverseFromEnd)
    (:Update
      (Transformation|SetRelativeLocation (Variables|Default|GetStaticMesh) (Math|Vector|MakeVector 0.0 0.0 (* _newtrack_0 1e+02)) false false))
    (:Finished
      (if (Utilities|Enum|Equal(Enum) _direction "Forward")
        (CallFunction|PlayBackward)
        (else
          (CallFunction|PlayForward))))))

(event EventBeginPlay
  (bind (_direction _newtrack_0) (Timeline|Timeline Play)
    (:Update
      (Transformation|SetRelativeLocation (Variables|Default|GetStaticMesh) (Math|Vector|MakeVector 0.0 0.0 (* _newtrack_0 1e+02)) false false))
    (:Finished
      (if (Utilities|Enum|Equal(Enum) _direction "Forward")
        (CallFunction|PlayBackward)
        (else
          (CallFunction|PlayForward))))))

(event Collision|EventActorBeginOverlap
  (params (OtherActor :type Actor%20Object%20Reference)))

(event EventTick
  (params (DeltaSeconds :type Float%20%28single-precision%29)))

(fn ConstructionScript)